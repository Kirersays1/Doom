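; Base enemy Blueprint that renders as a directional Paper2D sprite, with melee and ranged attacks.
; Tick derives an idle, move or attack state, then picks that state's flipbook and rotation from the player's angle via dot products.
; Pawn sensing and damage set a blackboard sight flag and turn it toward the player.
; Melee uses a line trace, ranged spawns a projectile, and death stops AI and collision before playing death flipbooks.
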(event OnSeePawn(PawnSensing)
  (params (Pawn :type Pawn%20Object%20Reference))
  ;[1 1 1] SeePlayer
  (Utilities|Casting|CastToBP_FirstPersonCharacter Pawn)
  (Variables|NoEdit|Setcansee true)
  (AI|Components|Blackboard|SetValueasBool (AI|GetBlackboard 0) (Utilities|Name|MakeLiteralName "canseeplayer") true)
  (Utilities|FlowControl|RetriggerableDelay 0.7)
  (Variables|NoEdit|Setcansee false)
  (AI|Components|Blackboard|SetValueasBool (AI|GetBlackboard 0) (Utilities|Name|MakeLiteralName "canseeplayer") false))

(event Custom|RotatetoPlayer
  ;[1 1 1] SeePlayer
  (Transformation|SetActorRotation (Math|Interpolation|RInterpTo (Transformation|GetActorRotation) (Math|Rotator|FindLookatRotation (Transformation|GetActorLocation) (Transformation|GetActorLocation (Game|GetPlayerCharacter 0))) (Utilities|Time|GetWorldDeltaSeconds) (Variables|Edit|GetRotationSpeed))))

(event Custom|SpawnProjectile
  ;[1 1 1] RangeAttack
  (Variables|NoEdit|SetisAttack true)
  (Variables|NoEdit|Setattackstate "NewEnumerator1")
  (Components|Movement|StopMovementImmediately (Variables|Character|GetCharacterMovement))
  (Game|SpawnActorfromClass "/Game/Blueprints/Projectiles/BP_EnemyProjectile.BP_EnemyProjectile_C" (Transformation|GetWorldTransform (Variables|Default|Getprojectilespawn)) "Undefined" 0 (Variables|Edit|GetprojectileSpeed) (Variables|Edit|GetprojectileDamage) 0)
  (Utilities|FlowControl|RetriggerableDelay (+ (Variables|Edit|GetfireRate) 0.1))
  (Variables|NoEdit|SetisAttack false))

(event Custom|MeleeAttack
  (bind _returnvalue (Transformation|GetActorLocation))
  ;[1 1 1] MeleeAttack
  (Variables|NoEdit|SetisAttack true)
  (Variables|NoEdit|Setattackstate "NewEnumerator0")
  (bind _outhit (Collision|LineTraceForObjects _returnvalue (+ _returnvalue (* (Transformation|GetActorForwardVector) 1.5e+02)) (Utilities|Array|MakeArray "ObjectTypeQuery3") false (Utilities|Array|MakeArray self) "ForDuration"))
  (if (== (.HitActor (Collision|BreakHitResult _outhit)) (Game|GetPlayerCharacter 0))
    (Game|Damage|ApplyDamage (.HitActor (Collision|BreakHitResult _outhit)) (Variables|Edit|GetEnemyDamage) 0 0)
    (Audio|PlaySoundatLocation "/Game/Audio/VFX/Mons1.Mons1" "0, 0, 0" "0, 0, 0" 1.0 1.0 0.0 0 0 0 0))
  (Utilities|FlowControl|RetriggerableDelay (+ (Variables|Edit|GetmeleeRate) 0.1))
  (Variables|NoEdit|SetisAttack false))

(event Custom|Death
  (bind _paperflipbook (Variables|Default|GetPaperFlipbook))
  ;[1 1 1] Death Flipbook
  (Transformation|SetActorRotation (Math|Rotator|MakeRotator 0.0 0.0 (.yaw (Math|Rotator|FindLookatRotation (Transformation|GetActorLocation) (Transformation|GetActorLocation (Game|GetPlayerCharacter 0))))))
  (Utilities|FlowControl|DoOnce false
    (:Completed
      (AI|Logic|StopLogic (Variables|/Script/AIModule.AIController|GetBrainComponent (AI|GetAIController self)) "")
      (Pawn|Components|CharacterMovement|SetMovementMode (Variables|Character|GetCharacterMovement) "MOVE_Flying" 0)
      (Collision|SetCollisionEnabled (Variables|Collision|GetCapsuleComponent) "NoCollision")
      (Components|Activation|Deactivate (Variables|Character|GetCharacterMovement))
      (Transformation|SetRelativeRotation _paperflipbook "0.000000,-90.000000,0.000000" false false)
      (Sprite|SetFlipbook _paperflipbook (Variables|Edit|GetenemyDeath_FB))
      (Utilities|FlowControl|Delay (- (Class|PaperFlipbookComponent|GetFlipbookLength _paperflipbook) 0.2))
      (Transformation|AddActorLocalOffset "0.000000,0.000000,-50.000000" false false)
      (Sprite|SetFlipbook _paperflipbook (Variables|Edit|GetenemyDeathIdle_FB)))))

(event Game|Damage|EventAnyDamage
  (params (Damage :type Float%20%28single-precision%29) (DamageType :type Damage%20Type%20Object%20Reference) (InstigatedBy :type Controller%20Object%20Reference) (DamageCauser :type Actor%20Object%20Reference))
  ;[1 1 1] EnemyDamage
  (bind _output_get (Variables|Edit|Sethealth (- (Variables|Edit|Gethealth) Damage)))
  (if (<= _output_get 0.0)
    (Variables|NoEdit|SetisDead true)
    (else
      ;[1 1 1] turnToDamage
      (Variables|NoEdit|Setcansee true)
      (AI|Components|Blackboard|SetValueasBool (AI|GetBlackboard 0) (Utilities|Name|MakeLiteralName "canseeplayer") true))))

(event EventTick
  (params (DeltaSeconds :type Float%20%28single-precision%29))
  (bind _returnvalue (Game|GetPlayerCharacter 0))
  (bind _returnvalue_2 (Transformation|GetActorLocation))
  (bind _isattack (Variables|NoEdit|GetisAttack))
  (bind _attackstate (Variables|NoEdit|Getattackstate))
  (bind _returnvalue_3 (Transformation|GetActorLocation _returnvalue))
  (bind _returnvalue_4 (- _returnvalue_3 _returnvalue_2))
  (bind _returnvalue_5 (Math|Vector|Normalize _returnvalue_4))
  (if (> (Math|Vector|VectorLength (Variables|/Script/Engine.MovementComponent|GetVelocity (Variables|Character|GetCharacterMovement))) 0.0)
    (if _isattack
      (switch Utilities|FlowControl|Switch|SwitchonAttackStatus_Enum _attackstate
        (:NewEnumerator0
          (Variables|NoEdit|Setenemystate "NewEnumerator2"))
        (:NewEnumerator1
          (Variables|NoEdit|Setenemystate "NewEnumerator3")))
      (else
        (Variables|NoEdit|Setenemystate "NewEnumerator1")))
    (elif _isattack
      (switch Utilities|FlowControl|Switch|SwitchonAttackStatus_Enum _attackstate
        (:NewEnumerator0
          (Variables|NoEdit|Setenemystate "NewEnumerator2"))
        (:NewEnumerator1
          (Variables|NoEdit|Setenemystate "NewEnumerator3")))
      (else
        (Variables|NoEdit|Setenemystate "NewEnumerator0"))))
  (if (Variables|NoEdit|GetisDead)
    (CallFunction|Death)
    (else
      (if (Variables|NoEdit|Getcansee)
        (CallFunction|RotatetoPlayer))
      ;[1 1 1] EnemyFacingDirection| Player Reference
      (Variables|NoEdit|Setdegrees (Class|KismetMathLibrary|DegAcos (Math|Vector|DotProduct (Transformation|GetActorForwardVector) _returnvalue_5)))
      (if (< (Math|Vector|DotProduct (Transformation|GetActorRightVector) _returnvalue_5) 0.0)
        (Math|Float|CompareFloat (Variables|NoEdit|Getdegrees) 1.8e+02
          (:>
            (Transformation|SetRelativeRotation (Variables|Default|GetPaperFlipbook) "0.000000,-90.000000,0.000000" false false :!label _label)
            (Sprite|SetFlipbook (Variables|Default|GetPaperFlipbook) (Utilities|Array|Get(acopy) (Utilities|Select :Index (Variables|NoEdit|Getenemystate) :NewEnumerator0 (Variables|Flipbooks|GetflipbooksIdle) :NewEnumerator1 (Variables|Flipbooks|GetflipbooksMove) :NewEnumerator2 (Variables|Flipbooks|GetflipbooksMelee) :NewEnumerator3 (Variables|Flipbooks|GetflibooksRange)))))
          (:==
            (goto _label))
          (:<
            (Math|Float|CompareFloat (Variables|NoEdit|Getdegrees) 135.0
              (:>
                (Transformation|SetRelativeRotation (Variables|Default|GetPaperFlipbook) "0.000000,135.000000,0.000000" false false :!label _label_2)
                (Sprite|SetFlipbook (Variables|Default|GetPaperFlipbook) (Utilities|Array|Get(acopy) (Utilities|Select :Index (Variables|NoEdit|Getenemystate) :NewEnumerator0 (Variables|Flipbooks|GetflipbooksIdle) :NewEnumerator1 (Variables|Flipbooks|GetflipbooksMove) :NewEnumerator2 (Variables|Flipbooks|GetflipbooksMelee) :NewEnumerator3 (Variables|Flipbooks|GetflibooksRange)) 3)))
              (:==
                (goto _label_2))
              (:<
                (Math|Float|CompareFloat (Variables|NoEdit|Getdegrees) 9e+01
                  (:>
                    (Transformation|SetRelativeRotation (Variables|Default|GetPaperFlipbook) "0.000000,180.000000,0.000000" false false :!label _label_3)
                    (Sprite|SetFlipbook (Variables|Default|GetPaperFlipbook) (Utilities|Array|Get(acopy) (Utilities|Select :Index (Variables|NoEdit|Getenemystate) :NewEnumerator0 (Variables|Flipbooks|GetflipbooksIdle) :NewEnumerator1 (Variables|Flipbooks|GetflipbooksMove) :NewEnumerator2 (Variables|Flipbooks|GetflipbooksMelee) :NewEnumerator3 (Variables|Flipbooks|GetflibooksRange)) 2)))
                  (:==
                    (goto _label_3))
                  (:<
                    (Math|Float|CompareFloat (Variables|NoEdit|Getdegrees) 45.0
                      (:>
                        _)
                      (:==
                        _)
                      (:<
                        (goto _label)))
                    (Transformation|SetRelativeRotation (Variables|Default|GetPaperFlipbook) "0.000000,45.000000,0.000000" false false)
                    (Sprite|SetFlipbook (Variables|Default|GetPaperFlipbook) (Utilities|Array|Get(acopy) (Utilities|Select :Index (Variables|NoEdit|Getenemystate) :NewEnumerator0 (Variables|Flipbooks|GetflipbooksIdle) :NewEnumerator1 (Variables|Flipbooks|GetflipbooksMove) :NewEnumerator2 (Variables|Flipbooks|GetflipbooksMelee) :NewEnumerator3 (Variables|Flipbooks|GetflibooksRange)) 1))))))))
        (else
          (Math|Float|CompareFloat (Variables|NoEdit|Getdegrees) 1.8e+02
            (:>
              (Transformation|SetRelativeRotation (Variables|Default|GetPaperFlipbook) "0.000000,-45.000000,0.000000" false false :!label _label_4)
              (Sprite|SetFlipbook (Variables|Default|GetPaperFlipbook) (Utilities|Array|Get(acopy) (Utilities|Select :Index (Variables|NoEdit|Getenemystate) :NewEnumerator0 (Variables|Flipbooks|GetflipbooksIdle) :NewEnumerator1 (Variables|Flipbooks|GetflipbooksMove) :NewEnumerator2 (Variables|Flipbooks|GetflipbooksMelee) :NewEnumerator3 (Variables|Flipbooks|GetflibooksRange)))))
            (:==
              (goto _label_4))
            (:<
              (Math|Float|CompareFloat (Variables|NoEdit|Getdegrees) 135.0
                (:>
                  (Transformation|SetRelativeRotation (Variables|Default|GetPaperFlipbook) "0.000000,90.000000,0.000000" false false :!label _label_5)
                  (Sprite|SetFlipbook (Variables|Default|GetPaperFlipbook) (Utilities|Array|Get(acopy) (Utilities|Select :Index (Variables|NoEdit|Getenemystate) :NewEnumerator0 (Variables|Flipbooks|GetflipbooksIdle) :NewEnumerator1 (Variables|Flipbooks|GetflipbooksMove) :NewEnumerator2 (Variables|Flipbooks|GetflipbooksMelee) :NewEnumerator3 (Variables|Flipbooks|GetflibooksRange)) 4)))
                (:==
                  (goto _label_5))
                (:<
                  (Math|Float|CompareFloat (Variables|NoEdit|Getdegrees) 9e+01
                    (:>
                      (Transformation|SetRelativeRotation (Variables|Default|GetPaperFlipbook) "0.000000,-90.000000,0.000000" false false :!label _label_6)
                      (Sprite|SetFlipbook (Variables|Default|GetPaperFlipbook) (Utilities|Array|Get(acopy) (Utilities|Select :Index (Variables|NoEdit|Getenemystate) :NewEnumerator0 (Variables|Flipbooks|GetflipbooksIdle) :NewEnumerator1 (Variables|Flipbooks|GetflipbooksMove) :NewEnumerator2 (Variables|Flipbooks|GetflipbooksMelee) :NewEnumerator3 (Variables|Flipbooks|GetflibooksRange)) 5)))
                    (:==
                      (goto _label_6))
                    (:<
                      (Math|Float|CompareFloat (Variables|NoEdit|Getdegrees) 45.0
                        (:>
                          _)
                        (:==
                          _)
                        (:<
                          (goto _label_4)))
                      (Transformation|SetRelativeRotation (Variables|Default|GetPaperFlipbook) "0, 0, 0" false false)
                      (Sprite|SetFlipbook (Variables|Default|GetPaperFlipbook) (Utilities|Array|Get(acopy) (Utilities|Select :Index (Variables|NoEdit|Getenemystate) :NewEnumerator0 (Variables|Flipbooks|GetflipbooksIdle) :NewEnumerator1 (Variables|Flipbooks|GetflipbooksMove) :NewEnumerator2 (Variables|Flipbooks|GetflipbooksMelee) :NewEnumerator3 (Variables|Flipbooks|GetflibooksRange)) 6)))))))))))))

(fn ConstructionScript)