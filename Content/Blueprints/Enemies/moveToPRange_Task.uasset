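; Behavior tree task that moves an enemy pawn toward player 0 to bring it within range.
; On execute, it measures the pawn's distance to the player and fails immediately if that is 1000 units or less.
; Otherwise it runs AIMoveTo on the player with a much larger 7500-unit acceptance radius, finishing successfully when the move succeeds.
; A failed move never calls FinishExecute, leaving the task running.
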(event EventReceiveExecuteAI
  (params (OwnerController :type AI%20Controller%20Object%20Reference) (ControlledPawn :type Pawn%20Object%20Reference))
  (if (> (Math|Vector|VectorLength (- (Transformation|GetActorLocation ControlledPawn) (Transformation|GetActorLocation (Game|GetPlayerCharacter 0)))) 1e+03)
    (AI|AIMoveTo ControlledPawn "0, 0, 0" (Game|GetPlayerCharacter 0) 7.5e+03 false
      (:OnSuccess
        (AI|BehaviorTree|FinishExecute true)))
    (else
      (AI|BehaviorTree|FinishExecute false))))