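; Locked door that opens when the first-person player enters its box while carrying the matching gold, green or red key.
; The Key enum picks both the cube's material in the construction script and which character key flag is checked on overlap.
; A match fires once, running a timeline that raises the cube by lerping from its current height each update, then destroys the actor after a short delay.
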(event OnComponentBeginOverlap(Box)
  (params (OverlappedComponent :type Primitive%20Component%20Object%20Reference) (OtherActor :type Actor%20Object%20Reference) (OtherComp :type Primitive%20Component%20Object%20Reference) (OtherBodyIndex :type Integer) (bFromSweep :type Boolean) (SweepResult :type Hit%20Result%20Structure%20%28by%20ref%29))
  (bind _cube (Variables|Default|GetCube))
  (bind _returnvalue (Transformation|GetWorldLocation _cube))
  (bind _asbp_first_person_character (Utilities|Casting|CastToBP_FirstPersonCharacter OtherActor))
  (Variables|Default|SetAs%20BP%20First%20Person%20Character _asbp_first_person_character)
  (switch Utilities|FlowControl|Switch|Switchonkeys (Variables|Default|Getkey)
    (:NewEnumerator0
      (if (Variables|/Game/FirstPerson/Blueprints/BP_FirstPersonCharacter.BP_FirstPersonCharacter_C|GetgoldKey? (Variables|Default|GetAs%20BP%20First%20Person%20Character))
        (Utilities|FlowControl|DoOnce false :!label _label
          (:Completed
            (bind _newtrack_0 (Timeline|Timeline_0 PlayFromStart)
              (:Update
                (Transformation|SetWorldLocation _cube (Math|Vector|MakeVector (.x _returnvalue) (.y _returnvalue) (Math|Float|Lerp (.z _returnvalue) (+ (.z _returnvalue) 15.0) _newtrack_0)) false false))
              (:Finished
                (Utilities|FlowControl|Delay 0.2)
                (Actor|DestroyActor)))))))
    (:NewEnumerator1
      (if (Variables|/Game/FirstPerson/Blueprints/BP_FirstPersonCharacter.BP_FirstPersonCharacter_C|Getgreenkey? (Variables|Default|GetAs%20BP%20First%20Person%20Character))
        (goto _label)))
    (:NewEnumerator2
      (if (Variables|/Game/FirstPerson/Blueprints/BP_FirstPersonCharacter.BP_FirstPersonCharacter_C|GetredKey? (Variables|Default|GetAs%20BP%20First%20Person%20Character))
        (goto _label)))))

(event EventBeginPlay)

(event Collision|EventActorBeginOverlap
  (params (OtherActor :type Actor%20Object%20Reference)))

(fn ConstructionScript
  (bind _cube (Variables|Default|GetCube))
  (switch Utilities|FlowControl|Switch|Switchonkeys (Variables|Default|Getkey)
    (:NewEnumerator0
      (Rendering|Material|SetMaterial _cube 0 "/Game/StarterContent/Materials/M_Metal_Gold.M_Metal_Gold"))
    (:NewEnumerator1
      (Rendering|Material|SetMaterial _cube 0 "/Engine/EngineDebugMaterials/VertexColorViewMode_GreenOnly.VertexColorViewMode_GreenOnly"))
    (:NewEnumerator2
      (Rendering|Material|SetMaterial _cube 0 "/Engine/VREditor/LaserPointer/LaserPointerMaterial.LaserPointerMaterial"))))