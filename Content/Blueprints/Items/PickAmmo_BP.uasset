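; Ammo pickup shown as a Paper2D sprite that billboards on yaw toward the player every tick.
; Construction script applies Ammo_Sprite, the same variable for every Ammotype.
; On box overlap by BP_FirstPersonCharacter, a DoOnce adds AmmoGive to the Bullet, Shell, Rocket or Cell count, clamped to its max, and updates the HUD.
; The actor then destroys itself, except in the Shell case, which has no destroy call.
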(event OnComponentBeginOverlap(Box)
  (params (OverlappedComponent :type Primitive%20Component%20Object%20Reference) (OtherActor :type Actor%20Object%20Reference) (OtherComp :type Primitive%20Component%20Object%20Reference) (OtherBodyIndex :type Integer) (bFromSweep :type Boolean) (SweepResult :type Hit%20Result%20Structure%20%28by%20ref%29))
  (bind _asbp_first_person_character (Utilities|Casting|CastToBP_FirstPersonCharacter OtherActor))
  (Variables|Default|SetAs%20BP%20First%20Person%20Character _asbp_first_person_character)
  (Utilities|FlowControl|DoOnce false
    (:Completed
      (switch Utilities|FlowControl|Switch|SwitchonAmmotype (Variables|Default|Getammotype)
        (:NewEnumerator0
          ;[1 1 1] GiveBullet
          (Variables|/Game/FirstPerson/Blueprints/BP_FirstPersonCharacter.BP_FirstPersonCharacter_C|Setbullet (Variables|Default|GetAs%20BP%20First%20Person%20Character) (Math|Integer|Clamp(Integer) (+ (Variables|/Game/FirstPerson/Blueprints/BP_FirstPersonCharacter.BP_FirstPersonCharacter_C|Getbullet (Variables|Default|GetAs%20BP%20First%20Person%20Character)) (Variables|Default|GetammoGive)) 0 (Variables|/Game/FirstPerson/Blueprints/BP_FirstPersonCharacter.BP_FirstPersonCharacter_C|GetmaxBullet (Variables|Default|GetAs%20BP%20First%20Person%20Character))))
          (Default|UpdateBullet (Variables|/Game/FirstPerson/Blueprints/BP_FirstPersonCharacter.BP_FirstPersonCharacter_C|Getplayerhud (Variables|Default|GetAs%20BP%20First%20Person%20Character)))
          (Actor|DestroyActor))
        (:NewEnumerator1
          ;[1 1 1] GiveShell
          (Variables|/Game/FirstPerson/Blueprints/BP_FirstPersonCharacter.BP_FirstPersonCharacter_C|Setshell (Variables|Default|GetAs%20BP%20First%20Person%20Character) (Math|Integer|Clamp(Integer) (+ (Variables|/Game/FirstPerson/Blueprints/BP_FirstPersonCharacter.BP_FirstPersonCharacter_C|Getshell (Variables|Default|GetAs%20BP%20First%20Person%20Character)) (Variables|Default|GetammoGive)) 0 (Variables|/Game/FirstPerson/Blueprints/BP_FirstPersonCharacter.BP_FirstPersonCharacter_C|GetmaxShell (Variables|Default|GetAs%20BP%20First%20Person%20Character))))
          (Default|UpdateShell (Variables|/Game/FirstPerson/Blueprints/BP_FirstPersonCharacter.BP_FirstPersonCharacter_C|Getplayerhud (Variables|Default|GetAs%20BP%20First%20Person%20Character))))
        (:NewEnumerator2
          ;[1 1 1] GiveRock
          (Variables|/Game/FirstPerson/Blueprints/BP_FirstPersonCharacter.BP_FirstPersonCharacter_C|Setrock (Variables|Default|GetAs%20BP%20First%20Person%20Character) (Math|Integer|Clamp(Integer) (+ (Variables|/Game/FirstPerson/Blueprints/BP_FirstPersonCharacter.BP_FirstPersonCharacter_C|Getrock (Variables|Default|GetAs%20BP%20First%20Person%20Character)) (Variables|Default|GetammoGive)) 0 (Variables|/Game/FirstPerson/Blueprints/BP_FirstPersonCharacter.BP_FirstPersonCharacter_C|GetmaxRock (Variables|Default|GetAs%20BP%20First%20Person%20Character))))
          (Default|UpdateRocket (Variables|/Game/FirstPerson/Blueprints/BP_FirstPersonCharacter.BP_FirstPersonCharacter_C|Getplayerhud (Variables|Default|GetAs%20BP%20First%20Person%20Character)))
          (Actor|DestroyActor))
        (:NewEnumerator3
          ;[1 1 1] Cell
          (Variables|/Game/FirstPerson/Blueprints/BP_FirstPersonCharacter.BP_FirstPersonCharacter_C|Setcell (Variables|Default|GetAs%20BP%20First%20Person%20Character) (Math|Integer|Clamp(Integer) (+ (Variables|/Game/FirstPerson/Blueprints/BP_FirstPersonCharacter.BP_FirstPersonCharacter_C|Getcell (Variables|Default|GetAs%20BP%20First%20Person%20Character)) (Variables|Default|GetammoGive)) 0 (Variables|/Game/FirstPerson/Blueprints/BP_FirstPersonCharacter.BP_FirstPersonCharacter_C|GetmaxCell (Variables|Default|GetAs%20BP%20First%20Person%20Character))))
          (Default|UpdateCell (Variables|/Game/FirstPerson/Blueprints/BP_FirstPersonCharacter.BP_FirstPersonCharacter_C|Getplayerhud (Variables|Default|GetAs%20BP%20First%20Person%20Character)))
          (Actor|DestroyActor))))))

(event EventBeginPlay)

(event Collision|EventActorBeginOverlap
  (params (OtherActor :type Actor%20Object%20Reference)))

(event EventTick
  (params (DeltaSeconds :type Float%20%28single-precision%29))
  (Transformation|SetActorRotation (Math|Rotator|MakeRotator 0.0 0.0 (.yaw (Math|Rotator|FindLookatRotation (Transformation|GetActorLocation) (Transformation|GetActorLocation (Game|GetPlayerCharacter 0)))))))

(fn ConstructionScript
  (bind _papersprite (Variables|Default|GetPaperSprite))
  (switch Utilities|FlowControl|Switch|SwitchonAmmotype (Variables|Default|Getammotype)
    (:NewEnumerator0
      (Rendering|Components|Sprite|SetSprite _papersprite "/Game/Sprites/Items/Ammo_Sprite.Ammo_Sprite"))
    (:NewEnumerator1
      (Rendering|Components|Sprite|SetSprite _papersprite "/Game/Sprites/Items/Ammo_Sprite.Ammo_Sprite"))
    (:NewEnumerator2
      (Rendering|Components|Sprite|SetSprite _papersprite "/Game/Sprites/Items/Ammo_Sprite.Ammo_Sprite"))
    (:NewEnumerator3
      (Rendering|Components|Sprite|SetSprite _papersprite "/Game/Sprites/Items/Ammo_Sprite.Ammo_Sprite"))))