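; Sprite actor that displays a configurable Paper2D sprite as a billboard item facing the player.
; The construction script applies the chosen sprite and scale to its PaperSprite component.
; Every tick it turns to the player character using only the yaw of a look-at rotation, so it stays upright.
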(event EventBeginPlay)

(event Collision|EventActorBeginOverlap
  (params (OtherActor :type Actor%20Object%20Reference)))

(event EventTick
  (params (DeltaSeconds :type Float%20%28single-precision%29))
  (Transformation|SetActorRotation (Math|Rotator|MakeRotator 0.0 0.0 (.yaw (Math|Rotator|FindLookatRotation (Transformation|GetActorLocation) (Transformation|GetActorLocation (Game|GetPlayerCharacter 0)))))))

(fn ConstructionScript
  (bind _papersprite (Variables|Default|GetPaperSprite))
  (Rendering|Components|Sprite|SetSprite _papersprite (Variables|Default|GetSpriteC))
  (Transformation|SetWorldScale3D _papersprite (Variables|Default|GetScale)))