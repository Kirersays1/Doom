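; Key pickup actor that grants the first-person player a gold, green or red key, depending on its Key enum.
; The construction script sets the Paper2D sprite to match the key type.
; On Tick the actor yaws to face the player, billboard-style.
; Box overlap by BP_FirstPersonCharacter sets the matching key flag, calls that key's Find function on the player HUD, and destroys the pickup.
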(event OnComponentBeginOverlap(Box)
  (params (OverlappedComponent :type Primitive%20Component%20Object%20Reference) (OtherActor :type Actor%20Object%20Reference) (OtherComp :type Primitive%20Component%20Object%20Reference) (OtherBodyIndex :type Integer) (bFromSweep :type Boolean) (SweepResult :type Hit%20Result%20Structure%20%28by%20ref%29))
  (bind _asbp_first_person_character (Utilities|Casting|CastToBP_FirstPersonCharacter OtherActor))
  (Variables|Default|SetAs%20BP%20First%20Person%20Character _asbp_first_person_character)
  (switch Utilities|FlowControl|Switch|Switchonkeys (Variables|Default|Getkey)
    (:NewEnumerator0
      (Variables|/Game/FirstPerson/Blueprints/BP_FirstPersonCharacter.BP_FirstPersonCharacter_C|SetgoldKey? (Variables|Default|GetAs%20BP%20First%20Person%20Character) true)
      (Default|FindGoldKey (Variables|/Game/FirstPerson/Blueprints/BP_FirstPersonCharacter.BP_FirstPersonCharacter_C|Getplayerhud (Variables|Default|GetAs%20BP%20First%20Person%20Character)))
      (Actor|DestroyActor))
    (:NewEnumerator1
      (Variables|/Game/FirstPerson/Blueprints/BP_FirstPersonCharacter.BP_FirstPersonCharacter_C|Setgreenkey? (Variables|Default|GetAs%20BP%20First%20Person%20Character) true)
      (Default|FindGreenKey (Variables|/Game/FirstPerson/Blueprints/BP_FirstPersonCharacter.BP_FirstPersonCharacter_C|Getplayerhud (Variables|Default|GetAs%20BP%20First%20Person%20Character)))
      (Actor|DestroyActor))
    (:NewEnumerator2
      (Variables|/Game/FirstPerson/Blueprints/BP_FirstPersonCharacter.BP_FirstPersonCharacter_C|SetredKey? (Variables|Default|GetAs%20BP%20First%20Person%20Character) true)
      (Default|FindRedKey (Variables|/Game/FirstPerson/Blueprints/BP_FirstPersonCharacter.BP_FirstPersonCharacter_C|Getplayerhud (Variables|Default|GetAs%20BP%20First%20Person%20Character)))
      (Actor|DestroyActor))))

(event EventBeginPlay)

(event Collision|EventActorBeginOverlap
  (params (OtherActor :type Actor%20Object%20Reference)))

(event EventTick
  (params (DeltaSeconds :type Float%20%28single-precision%29))
  ;[1 1 1] FindActor
  (Transformation|SetActorRotation (Math|Rotator|MakeRotator 0.0 0.0 (.yaw (Math|Rotator|FindLookatRotation (Transformation|GetActorLocation) (Transformation|GetActorLocation (Game|GetPlayerCharacter 0)))))))

(fn ConstructionScript
  (bind _papersprite (Variables|Default|GetPaperSprite))
  (switch Utilities|FlowControl|Switch|Switchonkeys (Variables|Default|Getkey)
    (:NewEnumerator0
      (Rendering|Components|Sprite|SetSprite _papersprite "/Game/Sprites/Items/Key_Gold_Sprite.Key_Gold_Sprite"))
    (:NewEnumerator1
      (Rendering|Components|Sprite|SetSprite _papersprite "/Game/Sprites/Items/Key_Green_Sprite.Key_Green_Sprite"))
    (:NewEnumerator2
      (Rendering|Components|Sprite|SetSprite _papersprite "/Game/Sprites/Items/Key_Red_Sprite.Key_Red_Sprite"))))