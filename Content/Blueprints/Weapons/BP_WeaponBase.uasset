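; Base weapon Blueprint for the first-person character, with empty ShootWeapon and StopShooting events.
; FireWeapon does a hitscan line trace that applies damage and spawns blood on actors tagged enemy, while FireProjectile spawns a projectile with the weapon's speed and damage.
; EnoughAmmo and DecreaseAmmo switch on ammo type to check or reduce the character's matching ammo pool and refresh its HUD.
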(event Custom|ShootWeapon)

(event Custom|StopShooting)

(event Custom|DecreaseAmmo
  (bind _playercharacterreference (Variables|Default|GetPlayerCharacterReference))
  (bind _playercharacterreference_2 (Variables|Default|GetPlayerCharacterReference))
  (bind _playercharacterreference_3 (Variables|Default|GetPlayerCharacterReference))
  (bind _playercharacterreference_4 (Variables|Default|GetPlayerCharacterReference))
  ;[1 1 1] ReduceAmmo
  (switch Utilities|FlowControl|Switch|SwitchonAmmo (Variables|Default|GetammoType)
    (:NewEnumerator0
      ;;[1 1 1] Bullet
      (Math|Integer|DecrementInt (Variables|/Game/FirstPerson/Blueprints/BP_FirstPersonCharacter.BP_FirstPersonCharacter_C|Getbullet _playercharacterreference_3)
        (:%20%20
          (Default|UpdateBullet (Variables|/Game/FirstPerson/Blueprints/BP_FirstPersonCharacter.BP_FirstPersonCharacter_C|Getplayerhud _playercharacterreference_3)))))
    (:NewEnumerator1
      ;;[1 1 1] Shell
      (Math|Integer|DecrementInt (Variables|/Game/FirstPerson/Blueprints/BP_FirstPersonCharacter.BP_FirstPersonCharacter_C|Getshell _playercharacterreference_4)
        (:%20%20
          (Default|UpdateShell (Variables|/Game/FirstPerson/Blueprints/BP_FirstPersonCharacter.BP_FirstPersonCharacter_C|Getplayerhud _playercharacterreference_4)))))
    (:NewEnumerator2
      ;;[1 1 1] Rocket
      (Math|Integer|DecrementInt (Variables|/Game/FirstPerson/Blueprints/BP_FirstPersonCharacter.BP_FirstPersonCharacter_C|Getrock _playercharacterreference_2)
        (:%20%20
          (Default|UpdateRocket (Variables|/Game/FirstPerson/Blueprints/BP_FirstPersonCharacter.BP_FirstPersonCharacter_C|Getplayerhud _playercharacterreference_2)))))
    (:NewEnumerator3
      ;;[1 1 1] Cell
      (Math|Integer|DecrementInt (Variables|/Game/FirstPerson/Blueprints/BP_FirstPersonCharacter.BP_FirstPersonCharacter_C|Getcell _playercharacterreference)
        (:%20%20
          (Default|UpdateCell (Variables|/Game/FirstPerson/Blueprints/BP_FirstPersonCharacter.BP_FirstPersonCharacter_C|Getplayerhud _playercharacterreference)))))))

(event EventBeginPlay
  (bind _asbp_first_person_character (Utilities|Casting|CastToBP_FirstPersonCharacter (Game|GetPlayerCharacter 0)))
  (Variables|Default|SetPlayerCharacterReference _asbp_first_person_character))

(fn ConstructionScript)

(fn FireWeapon
  (bind _linetrace (Variables|Default|Getlinetrace))
  (bind _returnvalue (Transformation|GetWorldLocation _linetrace))
  (bind (_outhit _returnvalue_2) (Collision|LineTraceForObjects _returnvalue (+ _returnvalue (* (Math|Vector|GetForwardVector (Transformation|GetWorldRotation (Variables|Default|Getlinetrace))) (Variables|Default|GetlinetraceDistance))) (Utilities|Array|MakeArray "ObjectTypeQuery1" "ObjectTypeQuery2" "ObjectTypeQuery3") false (Utilities|Array|MakeArray self (Game|GetPlayerCharacter 0)) "ForDuration"))
  (if _returnvalue_2
    (Game|Damage|ApplyDamage (.HitActor (Collision|BreakHitResult _outhit)) (Variables|Default|GetWeaponDamage) 0 0)
    (if (Actor|ActorHasTag (.HitActor (Collision|BreakHitResult _outhit)) "enemy")
      (Game|SpawnActorfromClass "/Game/Sprites/EnemySprites/Blood/Blood_BP.Blood_BP_C" (Math|Transform|MakeTransform (.Location (Collision|BreakHitResult _outhit)) "0, 0, 0" "1.000000,1.000000,1.000000") "Undefined" 0 0))))

(fn EnoughAmmo
  (switch Utilities|FlowControl|Switch|SwitchonAmmo (Variables|Default|GetammoType)
    (:NewEnumerator0
      ;[1 1 1] Ammo
      (if (> (Variables|/Game/FirstPerson/Blueprints/BP_FirstPersonCharacter.BP_FirstPersonCharacter_C|Getbullet (Variables|Default|GetPlayerCharacterReference)) 0)
        (return true)
        (else
          (return false))))
    (:NewEnumerator1
      ;[1 1 1] Shell
      (if (> (Variables|/Game/FirstPerson/Blueprints/BP_FirstPersonCharacter.BP_FirstPersonCharacter_C|Getshell (Variables|Default|GetPlayerCharacterReference)) 0)
        (return true)
        (else
          (return false))))
    (:NewEnumerator2
      ;[1 1 1] Rocket
      (if (> (Variables|/Game/FirstPerson/Blueprints/BP_FirstPersonCharacter.BP_FirstPersonCharacter_C|Getrock (Variables|Default|GetPlayerCharacterReference)) 0)
        (return true)
        (else
          (return false))))
    (:NewEnumerator3
      ;[1 1 1] Cell
      (if (> (Variables|/Game/FirstPerson/Blueprints/BP_FirstPersonCharacter.BP_FirstPersonCharacter_C|Getcell (Variables|Default|GetPlayerCharacterReference)) 0)
        (return true)
        (else
          (return false))))))

(fn FireProjectile
  (Game|SpawnActorfromClass (Variables|Default|Getprojectile) (Transformation|GetWorldTransform (Variables|Default|GetprojectileTransform)) "Undefined" 0 (Variables|Default|GetprojectileSpeed) (Variables|Default|GetWeaponDamage) 0))