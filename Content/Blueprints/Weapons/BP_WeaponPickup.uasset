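; Weapon pickup actor that gives the first-person character a shotgun, minigun, RPG, chainsaw or plasma gun.
; The construction script uses the Weapon selection to set both the Paper2D sprite and the weapon class to grant.
; Sphere overlap by BP_FirstPersonCharacter passes that class to its Pickupweapon function, then destroys the pickup.
; Tick billboards the sprite by yawing the actor toward the player.
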(event OnComponentBeginOverlap(Sphere)
  (params (OverlappedComponent :type Primitive%20Component%20Object%20Reference) (OtherActor :type Actor%20Object%20Reference) (OtherComp :type Primitive%20Component%20Object%20Reference) (OtherBodyIndex :type Integer) (bFromSweep :type Boolean) (SweepResult :type Hit%20Result%20Structure%20%28by%20ref%29))
  ;[1 1 1] Pickup&Destroy
  (bind _asbp_first_person_character (Utilities|Casting|CastToBP_FirstPersonCharacter OtherActor))
  (Default|Pickupweapon _asbp_first_person_character (Variables|Default|GetWeaponClass))
  (Actor|DestroyActor))

(event EventBeginPlay)

(event Collision|EventActorBeginOverlap
  (params (OtherActor :type Actor%20Object%20Reference)))

(event EventTick
  (params (DeltaSeconds :type Float%20%28single-precision%29))
  ;[1 1 1] Make Weapon Follow Rotation
  (Transformation|SetActorRotation (Math|Rotator|MakeRotator 0.0 0.0 (.yaw (Math|Rotator|FindLookatRotation (Transformation|GetActorLocation) (Transformation|GetActorLocation (Game|GetPlayerCharacter 0)))))))

(fn ConstructionScript
  (switch Utilities|FlowControl|Switch|SwitchonWeapons (Variables|Default|GetWeapon)
    (:NewEnumerator0
      ;[1 1 1] Shotgun
      (Rendering|Components|Sprite|SetSprite (Variables|Default|GetPaperSprite) "/Game/Sprites/Weapons/Shotgun/Shotgun_Sprite.Shotgun_Sprite")
      (Variables|Default|SetWeaponClass "/Game/Blueprints/Weapons/BP_Weapon_Shotgun.BP_Weapon_Shotgun_C"))
    (:NewEnumerator1
      ;[1 1 1] Minigun
      (Rendering|Components|Sprite|SetSprite (Variables|Default|GetPaperSprite) "/Game/Sprites/Weapons/MiniGun/minigun_sprite.minigun_sprite")
      (Variables|Default|SetWeaponClass "/Game/Blueprints/Weapons/BP_Weapon_Minigun.BP_Weapon_Minigun_C"))
    (:NewEnumerator2
      ;[1 1 1] RPG
      (Rendering|Components|Sprite|SetSprite (Variables|Default|GetPaperSprite) "/Game/Sprites/Weapons/RPG/RPG_Sprite.RPG_Sprite")
      (Variables|Default|SetWeaponClass "/Game/Blueprints/Weapons/BP_Weapon_RPG.BP_Weapon_RPG_C"))
    (:NewEnumerator3
      ;[1 1 1] Chainsaw
      (Rendering|Components|Sprite|SetSprite (Variables|Default|GetPaperSprite) "/Game/Sprites/Weapons/Chainsaw/Chainsaw_Sprite.Chainsaw_Sprite")
      (Variables|Default|SetWeaponClass "/Game/Blueprints/Weapons/BP_Weapon_Chainsaw.BP_Weapon_Chainsaw_C"))
    (:NewEnumerator4
      ;[1 1 1] PlasmaGun
      (Rendering|Components|Sprite|SetSprite (Variables|Default|GetPaperSprite) "/Game/Sprites/Weapons/PlasmaGun/PlasmaGun_Sprite.PlasmaGun_Sprite")
      (Variables|Default|SetWeaponClass "/Game/Blueprints/Weapons/BP_Weapon_PlasmaRifle.BP_Weapon_PlasmaRifle_C"))))