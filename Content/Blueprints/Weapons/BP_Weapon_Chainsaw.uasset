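; Chainsaw weapon Blueprint that handles the start and stop of firing, using Paper2D flipbooks for its idle and shoot visuals.
; ShootWeapon passes a DoOnce gate and starts a short one-shot timer, which calls FireWeapon and switches to the shoot flipbook.
; StopShooting cancels any pending timer, restores the idle flipbook and resets the gate, so each press fires at most once.
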(event Custom|ResetChainsaw
  (Utilities|FlowControl|DoOnce false) ; enters at Reset
)

(event Custom|use%20chainsaw
  (CallFunction|FireWeapon)
  (Sprite|SetFlipbook (Variables|Default|GetWeaponFlipbook) "/Game/Sprites/Weapons/Chainsaw/Chainsaw_Shoot.Chainsaw_Shoot"))

(event EventStopShooting
  (Utilities|Time|ClearandInvalidateTimerbyHandle (Variables|Default|GetchainsawEvent))
  (Sprite|SetFlipbook (Variables|Default|GetWeaponFlipbook) "/Game/Sprites/Weapons/Chainsaw/Chainsaw_Idle.Chainsaw_Idle")
  (CallFunction|ResetChainsaw))

(event EventShootWeapon
  (Utilities|FlowControl|DoOnce false
    (:Completed
      (bind _returnvalue (Utilities|Time|SetTimerbyEvent (delegate Custom|use%20chainsaw) 0.15))
      (Variables|Default|SetchainsawEvent _returnvalue))))

(fn ConstructionScript
  (|CallParentFunction))