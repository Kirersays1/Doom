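; BP_Weapon_Fist is the fist weapon Blueprint, performing a punch attack when the weapon is fired.
; ShootWeapon passes through a DoOnce gate, calls FireWeapon, plays the Punch sound and switches the Paper2D flipbook to its shoot animation.
; After a delay equal to the flipbook's length, it restores the idle flipbook and calls ResetAttack to reopen the gate, blocking overlapping attacks.
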(event Custom|ResetAttack
  (bind _weaponflipbook (Variables|Default|GetWeaponFlipbook))
  (Utilities|FlowControl|DoOnce false) ; enters at Reset
)

(event EventShootWeapon
  (bind _weaponflipbook (Variables|Default|GetWeaponFlipbook))
  (Utilities|FlowControl|DoOnce false
    (:Completed
      (CallFunction|FireWeapon)
      (Audio|PlaySoundatLocation "/Game/Audio/VFX/punch.punch" "0, 0, 0" "0, 0, 0" 1.0 1.0 0.0 0 0 0 0)
      (Sprite|SetFlipbook _weaponflipbook "/Game/Sprites/Weapons/Punch/Weapon_Fist_Shoot.Weapon_Fist_Shoot")
      (Utilities|FlowControl|Delay (Class|PaperFlipbookComponent|GetFlipbookLength _weaponflipbook))
      (Sprite|SetFlipbook (Variables|Default|GetWeaponFlipbook) "/Game/Sprites/Weapons/Punch/Weapon_Fist_Idle.Weapon_Fist_Idle")
      (CallFunction|ResetAttack))))

(fn ConstructionScript
  (|CallParentFunction))