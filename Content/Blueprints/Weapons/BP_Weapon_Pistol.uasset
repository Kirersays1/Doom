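; Pistol weapon Blueprint, a child of a weapon base class, that handles firing with sound and a flipbook animation.
; ShootWeapon checks ammo, then passes through a DoOnce gate to decrease ammo, fire, play the pistol sound and switch to the fire flipbook.
; After a delay matching the flipbook's length, it restores the idle flipbook and ResetShoot reopens the gate, so the animation sets the fire rate.
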(event Custom|ResetShoot
  (bind _weaponflipbook (Variables|Default|GetWeaponFlipbook))
  (Utilities|FlowControl|DoOnce false) ; enters at Reset
)

(event EventShootWeapon
  (bind _weaponflipbook (Variables|Default|GetWeaponFlipbook))
  (bind _hasammo (CallFunction|EnoughAmmo))
  (if _hasammo
    (Utilities|FlowControl|DoOnce false
      (:Completed
        (CallFunction|DecreaseAmmo)
        (CallFunction|FireWeapon)
        (Audio|PlaySoundatLocation "/Game/Sprites/Weapons/Pistol/pistol.pistol" "0, 0, 0" "0, 0, 0" 1.0 1.0 0.0 0 0 0 0)
        (Sprite|SetFlipbook _weaponflipbook "/Game/Sprites/Weapons/Pistol/Weapon_Pistol_Fire.Weapon_Pistol_Fire")
        (Utilities|FlowControl|Delay (Class|PaperFlipbookComponent|GetFlipbookLength _weaponflipbook))
        (Sprite|SetFlipbook (Variables|Default|GetWeaponFlipbook) "/Game/Sprites/Weapons/Pistol/Weapon_Pistol_Idle.Weapon_Pistol_Idle")
        (CallFunction|ResetShoot)))))

(fn ConstructionScript
  (|CallParentFunction))