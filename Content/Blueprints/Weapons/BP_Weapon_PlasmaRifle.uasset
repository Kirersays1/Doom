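; Plasma rifle weapon Blueprint that fires projectiles automatically and switches its Paper2D flipbook between shoot and idle animations.
; ShootWeapon passes a DoOnce gate to start a looping timer on FireMinigun, which checks ammo, decrements it and fires a projectile.
; StopShooting or running out of ammo clears the timer and restores idle.
; The gate reopens only through the separate ResetFire event.
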(event Custom|FireMinigun
  (bind _hasammo (CallFunction|EnoughAmmo))
  (if _hasammo
    (CallFunction|DecreaseAmmo)
    (CallFunction|FireProjectile)
    (Sprite|SetFlipbook (Variables|Default|GetWeaponFlipbook) "/Game/Sprites/Weapons/PlasmaGun/PlasmaGun_Shoot.PlasmaGun_Shoot")
    (else
      (Utilities|Time|ClearandInvalidateTimerbyHandle (Variables|Default|Getminigunevent))
      (Sprite|SetFlipbook (Variables|Default|GetWeaponFlipbook) "/Game/Sprites/Weapons/PlasmaGun/PlasmaGun_Idle.PlasmaGun_Idle"))))

(event Custom|ResetFire
  (Utilities|FlowControl|DoOnce false) ; enters at Reset
)

(event EventShootWeapon
  (Utilities|FlowControl|DoOnce false
    (:Completed
      (bind _returnvalue (Utilities|Time|SetTimerbyEvent (delegate Custom|FireMinigun) 0.15 true))
      (Variables|Default|Setminigunevent _returnvalue))))

(event EventStopShooting
  (Utilities|Time|ClearandInvalidateTimerbyHandle (Variables|Default|Getminigunevent))
  (Sprite|SetFlipbook (Variables|Default|GetWeaponFlipbook) "/Game/Sprites/Weapons/PlasmaGun/PlasmaGun_Idle.PlasmaGun_Idle"))

(fn ConstructionScript
  (|CallParentFunction))