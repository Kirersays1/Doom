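; RPG weapon Blueprint that fires a projectile and plays a flipbook firing animation.
; ShootWeapon checks for ammo, then passes through a DoOnce gate to decrease ammo, fire the projectile and call FireWeapon.
; It swaps WeaponFlipbook to the shoot animation, delays for that flipbook's length, restores idle and calls ResetShoot to reopen the gate, so the animation length limits fire rate.
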(event Custom|ResetShoot
  (bind _weaponflipbook (Variables|Default|GetWeaponFlipbook))
  (Utilities|FlowControl|DoOnce false) ; enters at Reset
)

(event EventShootWeapon
  (bind _weaponflipbook (Variables|Default|GetWeaponFlipbook))
  (bind _hasammo (CallFunction|EnoughAmmo))
  (if _hasammo
    (Utilities|FlowControl|DoOnce false
      (:Completed
        (CallFunction|DecreaseAmmo)
        (CallFunction|FireProjectile)
        (CallFunction|FireWeapon)
        (Sprite|SetFlipbook _weaponflipbook "/Game/Sprites/Weapons/RPG/RPG_Shoot.RPG_Shoot")
        (Utilities|FlowControl|Delay (Class|PaperFlipbookComponent|GetFlipbookLength _weaponflipbook))
        (Sprite|SetFlipbook (Variables|Default|GetWeaponFlipbook) "/Game/Sprites/Weapons/RPG/RPG_Idle.RPG_Idle")
        (CallFunction|ResetShoot)))))

(fn ConstructionScript
  (|CallParentFunction))