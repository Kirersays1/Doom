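; Shotgun weapon Blueprint that fires with a sound and a Paper2D flipbook animation when enough ammo is available.
; ShootWeapon checks ammo, then passes a DoOnce gate to decrease ammo, fire, play the shot sound at world origin and show the fire flipbook.
; A delay matching the flipbook's length restores the idle flipbook and calls ResetShoot to reopen the gate, so the animation length sets the fire rate.
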(event Custom|ResetShoot
  (bind _weaponflipbook (Variables|Default|GetWeaponFlipbook))
  (Utilities|FlowControl|DoOnce false) ; enters at Reset
)

(event EventShootWeapon
  (bind _weaponflipbook (Variables|Default|GetWeaponFlipbook))
  (bind _hasammo (CallFunction|EnoughAmmo))
  (if _hasammo
    (Utilities|FlowControl|DoOnce false
      (:Completed
        (CallFunction|DecreaseAmmo)
        (CallFunction|FireWeapon)
        (Audio|PlaySoundatLocation "/Game/Audio/VFX/shotgun_shot.shotgun_shot" "0, 0, 0" "0, 0, 0" 1.0 1.0 0.0 0 0 0 0)
        (Sprite|SetFlipbook _weaponflipbook "/Game/Sprites/Weapons/Shotgun/Shotgun_Fire.Shotgun_Fire")
        (Utilities|FlowControl|Delay (Class|PaperFlipbookComponent|GetFlipbookLength _weaponflipbook))
        (Sprite|SetFlipbook (Variables|Default|GetWeaponFlipbook) "/Game/Sprites/Weapons/Shotgun/Shotgun_idle.Shotgun_idle")
        (CallFunction|ResetShoot)))))

(fn ConstructionScript
  (|CallParentFunction))